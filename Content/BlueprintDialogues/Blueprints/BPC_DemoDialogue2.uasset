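; BPC_DemoDialogue2 is a demo dialogue component that binds the dialogue system to its own data tables.
; Its lookup functions read dialogue row names and items from DT_DemoDialogue, speaker attributes from Speaker and asset references from Assest, reporting whether each row is found.
; It takes the script interpreter from FirstPersonGameMode.
; The data table functions are meant to be overridden by derived classes using other tables, and the event graph is empty.
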(event EventBeginPlay)

(event EventTick
  (params (DeltaSeconds :type Float%20%28single-precision%29)))

(fn GetScriptInterpreter
  (return (Variables|/Game/FirstPersonBP/Blueprints/FirstPersonGameMode.FirstPersonGameMode_C|GetScriptInterp (.AsFirst%20Person%20Game%20Mode (Utilities|Casting|CastToFirstPersonGameMode (Game|GetGameMode))))))

(fn GetDialogueRowNames
  ;[1 0 1] Override this function for derived classes using another data table
  (bind _outrownames (DataTable|GetDataTableRowNames "/Game/BlueprintDialogues/Data/DT_DemoDialogue.DT_DemoDialogue"))
  (return _outrownames))

(fn GetDialogueItem
  (params (ItemName :type Name))
  ;[1 0 1] Override this function for derived classes using another data table
  (bind _returnvalue (Utilities|GetDataTableRow "/Game/BlueprintDialogues/Data/DT_DemoDialogue.DT_DemoDialogue" ItemName)
    (:then
      (bind _result (Utilities|MakeBoolfromBranch :!label _label))
      (return _returnvalue _result))
    (:RowNotFound
      (goto _label False))))

(fn GetSpeakerAttributes
  (params (SpeakerID :type Name))
  ;[1 0 1] Override this function for derived classes using another data table
  (bind _returnvalue (Utilities|GetDataTableRow "/Game/BlueprintDialogues/Data/speaker.speaker" SpeakerID)
    (:then
      (bind _result (Utilities|MakeBoolfromBranch :!label _label))
      (return _returnvalue _result))
    (:RowNotFound
      (goto _label False))))

(fn GetAsset
  (params (ItemName :type Name))
  ;[1 0 1] Override this function for derived classes using another data table
  (bind _returnvalue (Utilities|GetDataTableRow "/Game/BlueprintDialogues/Data/assest.assest" ItemName)
    (:then
      (bind _result (Utilities|MakeBoolfromBranch :!label _label))
      (return _returnvalue _result))
    (:RowNotFound
      (goto _label False))))